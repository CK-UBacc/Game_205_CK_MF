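; Trigger zone actor that signals linked receiver actors when the player character overlaps it.
; It loops over the ReceiverActors set and sends SwitchTriggerMessage to each valid entry.
; TriggerOnce blocks firing while Triggered is set; otherwise every overlap fires.
; Triggered flips inside the loop once per valid receiver, so an even count leaves it unchanged and the one-shot can repeat.
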(event `self.ReceiveActorBeginOverlap`
  (params (OtherActor :type "Actor Object Reference"))
  (cast `/Game/Entities/Player/BP_Player_Character` OtherActor)
  (if (`self.TriggerOnce`)
    (if (not (`self.Triggered`))
      (bind _valuepin (`|SetForEach` (`self.ReceiverActors`) :!label _label)
        (:`then`
          (`/Engine/EditorBlueprintResources/StandardMacros.IsValid` _valuepin
            (:`Is Valid`
              (message `/Game/Interfaces/BPI_EnvironmentChange.SwitchTrigger` _valuepin)
              (set `self.Triggered` (not (`self.Triggered`))))))))
    (else
      (goto _label))))

(fn `UserConstructionScript`)