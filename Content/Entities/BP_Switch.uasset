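; Interactable switch that, on interact, sends SwitchTriggerMessage to every valid actor in its ReceiverActors set.
; TriggerOnce blocks interaction while Triggered is set; otherwise every interaction fires.
; Triggered flips inside the loop once per valid receiver, so its final state depends on how many there are.
; The dialogue, inventory and object-interaction functions are stubs returning fixed values.
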(event `/Game/Interfaces/BPI_Interaction.OnInteract`
  (params (InteractingChar :type "Character Object Reference"))
  (if (`self.TriggerOnce`)
    (if (not (`self.Triggered`))
      (bind _valuepin (`|SetForEach` (`self.ReceiverActors`) :!label _label)
        (:`then`
          (`/Engine/EditorBlueprintResources/StandardMacros.IsValid` _valuepin
            (:`Is Valid`
              (message `/Game/Interfaces/BPI_EnvironmentChange.SwitchTrigger` _valuepin)
              (set `self.Triggered` (not (`self.Triggered`))))))))
    (else
      (goto _label))))

(fn `AddToInventory`
  (params (ItemData :type "/Game/Entities/Pickups/PDA_PickupDataBase Object Reference"))
  (returns (Success :type Boolean))
  (return false))

(fn `GetDialogueText`
  (returns (DialogueText :type Text))
  (return "interact"))

(fn `HasDialogue`
  (returns (ShowDialogue :type Boolean))
  (return false))

(fn `InteractWithObject`
  (params (InteractingCharacter :type "Character Object Reference") (InteractingObject :type "/Game/Entities/Pickups/PDA_PickupDataBase Object Reference"))
  (returns (InteractionSuccess :type Boolean))
  (return false))

(fn `UserConstructionScript`)