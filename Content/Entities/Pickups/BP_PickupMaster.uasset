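; BP_PickupMaster is a pickup actor, named as the master for pickups, that the interacting character can add to their inventory.
; On interact, it sends that character an AddToInventory message carrying itself and its PickupName.
; It also answers interaction queries with a fixed interaction type and reports that it has dialogue, a "Press E to pick up" prompt built from PickupName.
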(event `/Game/Interfaces/BPI_Interaction.OnInteract`
  (params (InteractingChar :type "Character Object Reference"))
  (message `/Game/Interfaces/BPI_Interaction.AddToInventory` InteractingChar self (`self.PickupName`)))

(fn `GetDialogueText`
  (returns (DialogueText :type Text))
  (return (`|FormatText` "Press E to pick up {objName}" (`self.PickupName`))))

(fn `GetInteractionType`
  (returns (InteractType :type "/Game/ThirdPerson/Blueprints/E_InteractionType Enum"))
  (return "NewEnumerator2"))

(fn `HasDialogue`
  (returns (ShowDialogue :type Boolean))
  (return true))

(fn `UserConstructionScript`)