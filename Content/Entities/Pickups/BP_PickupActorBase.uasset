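; Base pickup actor whose item is defined by a PickupData asset.
; The construction script sets the static mesh from the asset's soft mesh reference when the data is valid.
; On interact, it passes the data to the interacting character's inventory message and destroys itself if that succeeds.
; Dialogue text builds a "pick up" prompt from the item name, while the other interaction, inventory and dialogue functions are stubs.
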(event `/Game/Interfaces/BPI_Interaction.OnInteract`
  (params (InteractingChar :type "Character Object Reference"))
  (bind _success (message `/Game/Interfaces/BPI_Interaction.AddToInventory` InteractingChar (`self.PickupData`)))
  (if _success
    (`self.K2_DestroyActor`)))

(fn `AddToInventory`
  (params (ItemData :type "/Game/Entities/Pickups/PDA_PickupDataBase Object Reference"))
  (returns (Success :type Boolean))
  (return false))

(fn `GetDialogueText`
  (returns (DialogueText :type Text))
  (return (`|FormatText` "pick up {name}" (`/Game/Entities/Pickups/PDA_PickupDataBase.ItemName` (`self.PickupData`)))))

(fn `GetNeedsItem`
  (returns (`NeedsItem?` :type Boolean))
  (return false))

(fn `HasDialogue`
  (returns (ShowDialogue :type Boolean))
  (return false))

(fn `InteractWithObject`
  (params (InteractingCharacter :type "Character Object Reference") (InteractingObject :type "/Game/Entities/Pickups/PDA_PickupDataBase Object Reference"))
  (returns (InteractionSuccess :type Boolean))
  (return false))

(fn `SetNeedsItem`
  (params (`NeedsItem?` :type Boolean))
  (return))

(fn `UserConstructionScript`
  (bind _pickupdata (`self.PickupData`) ; Check if Data asset is valid
    (:`then`
      (`StaticMeshComponent.SetStaticMesh` (`self.StaticMesh`) (`|ConvertAsset` (`/Game/Entities/Pickups/PDA_PickupDataBase.Mesh` _pickupdata))))
    (:`else`)))