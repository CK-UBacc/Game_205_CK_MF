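; BP_DoorSingle is an interactable, lockable single door that the player opens and closes.
; OnInteract toggles an unlocked door through an Actor Sequence, played forward to open and in reverse to close, or shows a "locked" dialogue popup.
; InteractWithObject compares an item's KeyID to the door's Key, unlocking and toggling the door on a match and printing debug text otherwise.
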(event `Actor Sequence Open Close Door`
  (params (`IsOpen?` :type Boolean))
  (bind _actorsequence (`self.ActorSequence`))
  (if `IsOpen?`
    (`MovieSceneSequencePlayer.PlayReverse` (`ActorSequenceComponent.SequencePlayer` _actorsequence))
    (set `self.Open` false)
    (else
      (`ActorSequenceComponent.PlaySequence` _actorsequence)
      (set `self.Open` true))))

(event `/Game/Interfaces/BPI_Interaction.OnInteract`
  (params (InteractingChar :type "Character Object Reference"))
  (bind _asbp_player_character (cast `/Game/Entities/Player/BP_Player_Character` InteractingChar))
  (if (`self.Unlocked?`)
    (`self.Actor Sequence Open Close Door` (`self.Open`))
    (else
      (`/Game/UI/BP_DialogueWDG.ShowDialogue` (`/Game/Entities/Player/BP_Player_Character.DialoguePopup` _asbp_player_character) "It's locked.  I need to find a key."))))

(fn `AddToInventory`
  (params (ItemData :type "/Game/Entities/Pickups/PDA_PickupDataBase Object Reference"))
  (returns (Success :type Boolean))
  (return false))

(fn `GetDialogueText`
  (returns (DialogueText :type Text))
  (return "try door"))

(fn `GetNeedsItem`
  (returns (`NeedsItem?` :type Boolean))
  (return (`self.NeedsItem?`)))

(fn `HasDialogue`
  (returns (ShowDialogue :type Boolean))
  (return false))

(fn `InteractWithObject`
  (params (InteractingCharacter :type "Character Object Reference") (InteractingObject :type "/Game/Entities/Pickups/PDA_PickupDataBase Object Reference"))
  (returns (InteractionSuccess :type Boolean))
  (bind _keyid (`/Game/Entities/Pickups/PDA_PickupDataBase.KeyID` InteractingObject))
  (bind _key (`self.Key`))
  (if (`KismetSystemLibrary.IsValid` InteractingObject)
    (if (`|EnumEquality` _keyid _key)
      (set `self.Unlocked?` true)
      (set `self.NeedsItem?` false)
      (`self.Actor Sequence Open Close Door` (`self.Open`))
      (return true)
      (else
        (`KismetSystemLibrary.PrintText` (`|FormatText` "Key ID: {id}" (`|GenericToText` _keyid)) true true (struct :`R` 1.0 :`G` 0.454282 :`A` 1.0))
        (`KismetSystemLibrary.PrintText` (`|FormatText` "Door Lock ID: {id}" (`|GenericToText` _key)) true true (struct :`R` 1.0 :`G` 0.454282 :`A` 1.0))
        (`KismetSystemLibrary.PrintText` "Key ID's do not match" true true (struct :`R` 1.0 :`G` 0.454282 :`A` 1.0))
        (return false)))
    (else
      (`KismetSystemLibrary.PrintText` "No item in inventory slot" true true (struct :`R` 1.0 :`G` 0.454282 :`A` 1.0)))))

(fn `UserConstructionScript`)