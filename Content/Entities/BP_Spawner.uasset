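; BP_Spawner is a trigger-driven actor that spawns a configurable class at its own transform.
; Each SwitchTrigger event spawns one instance of the class held in the Object variable.
; With TriggerOnce set, it then prints the spawned class and location on screen and destroys itself; otherwise it stays available for further triggers.
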(event `/Game/Interfaces/BPI_EnvironmentChange.SwitchTrigger`
  (bind _returnvalue (`self.GetTransform`))
  (bind _output (`|ConvertAsset` (`self.Object`)))
  (`|SpawnActorFromClass` _output _returnvalue "Undefined" "MultiplyWithRoot" null null)
  (if (`self.TriggerOnce`)
    (`KismetSystemLibrary.PrintText` (`|FormatText` "Spawned \"{actor} at \"{location}\"" (`KismetSystemLibrary.GetClassDisplayName` _output) (`KismetStringLibrary.Conv_VectorToString` (.location _returnvalue))) true true (struct :`G` 0.66 :`B` 1.0 :`A` 1.0) 5.0)
    (`self.K2_DestroyActor`)))

(fn `UserConstructionScript`)